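; FloorIsLava is a lava floor trap that damages the player and triggers a teleport on the socle.
; When anything overlaps the Lave component, it passes negative FloorDamages to player 0's GestionVie, then calls TPSocle on the BP_Socle found in the level.
; The overlapping actor is never checked, and leftover inline velocity-reset and teleport nodes are disconnected.
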(event `self.lave.OnComponentBeginOverlap`
  (params (OverlappedComponent :type "PrimitiveComponent Object Reference") (OtherActor :type "Actor Object Reference") (OtherComp :type "PrimitiveComponent Object Reference") (OtherBodyIndex :type Integer) (bFromSweep :type Boolean) (SweepResult :type "HitResult Structure (by ref)"))
  ;[1 1 1] Fall = death ?
  (bind _asfirst_person_character (cast `/Game/Blueprints/FirstPersonCharacter` (`GameplayStatics.GetPlayerCharacter` 0)))
  (`/Game/Blueprints/FirstPersonCharacter.GestionVie` _asfirst_person_character (* (`self.floorDamages`) -1))
  (bind _returnvalue (`GameplayStatics.GetActorOfClass` "/Game/Blueprints/Overboard/BP_Socle.BP_Socle_C"))
  (`/Game/Blueprints/Overboard/BP_Socle.TP_socle` _returnvalue))

(event `self.lave.OnComponentHit`
  (params (HitComponent :type "PrimitiveComponent Object Reference") (OtherActor :type "Actor Object Reference") (OtherComp :type "PrimitiveComponent Object Reference") (NormalImpulse :type "Vector Structure") (Hit :type "HitResult Structure (by ref)")))

(fn `UserConstructionScript`)