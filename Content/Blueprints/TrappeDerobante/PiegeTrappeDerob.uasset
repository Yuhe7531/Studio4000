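; Trapdoor trap actor whose grate gives way when the first-person character enters its trigger box.
; On the first overlap, a looping timer jitters the grate horizontally around its starting position for a configurable delay, with a door sound.
; It then resets the grate, disables the static frame's collision and drops the grate using physics with a mass override and falling-metal sound.
; The construction script removes the trigger when PiegeOrNot is false, leaving an inert trapdoor.
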(event `self.ReceiveBeginPlay`
  (set `self.Origine` (`SceneComponent.K2_GetComponentLocation` (`self.Grille`))))

(event `self.BoxPiege.OnComponentBeginOverlap`
  (params (OverlappedComponent :type "PrimitiveComponent Object Reference") (OtherActor :type "Actor Object Reference") (OtherComp :type "PrimitiveComponent Object Reference") (OtherBodyIndex :type Integer) (bFromSweep :type Boolean) (SweepResult :type "HitResult Structure (by ref)"))
  (bind _grille (`self.Grille`))
  (cast `/Game/Blueprints/FirstPersonCharacter` OtherActor)
  (`/Engine/EditorBlueprintResources/StandardMacros.DoOnce` false
    (:`Completed`
      (`GameplayStatics.PlaySound2D` "/Game/Partage/Audio/JailDoorOpen_Cue.JailDoorOpen_Cue" 1.0 1.0 0.0 null null)
      (`KismetSystemLibrary.K2_SetTimer` null "Tremblements" 0.05 true)
      (`KismetSystemLibrary.Delay` (`self.AttenteAvantDerob`))
      (`KismetSystemLibrary.K2_ClearTimer` null "Tremblements")
      (`SceneComponent.K2_SetWorldLocation` (`self.Grille`) (`self.Origine`) false false)
      (`GameplayStatics.PlaySound2D` "/Game/Partage/Audio/MetalFall_Cue.MetalFall_Cue" 1.0 1.0 0.0 null null)
      (`PrimitiveComponent.SetCollisionEnabled` (`self.CadreStatique`) "NoCollision")
      (`PrimitiveComponent.SetSimulatePhysics` _grille true)
      (`PrimitiveComponent.SetMassOverrideInKg` _grille "None" 100.0 true))))

(fn `Tremblements`
  (`SceneComponent.K2_SetWorldLocation` (`self.Grille`) (+ (`self.Origine`) (`KismetMathLibrary.MakeVector` (`KismetMathLibrary.RandomFloatInRange` -0.7 0.7) (`KismetMathLibrary.RandomFloatInRange` -0.7 0.7))) false false))

(fn `UserConstructionScript`
  (if (not (`self.PiegeOrNot`))
    (`ActorComponent.K2_DestroyComponent` (`self.BoxPiege`))))