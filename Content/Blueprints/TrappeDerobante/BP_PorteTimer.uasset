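; BP_PorteTimer is a door Blueprint whose OutTime event reveals LabDoor01 and slides it upward, apparently when a timer runs out.
; A DoOnce lets the sequence start only once.
; A looped short Delay then nudges the door up along world Z in unit steps, counted by EvolDoorPos until it reaches its limit.
; The CloseDoor function and construction script are empty.
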(event `/Game/Blueprints/DATA/BPI.OutTime`
  (bind _evoldoorpos (`self.evolDoorPos`))
  (bind _labdoor01 (`self.LabDoor01`))
  (`/Engine/EditorBlueprintResources/StandardMacros.DoOnce` false
    (:`Completed`
      (`SceneComponent.SetHiddenInGame` (`self.LabDoor01`) false false)
      (if (not (== _evoldoorpos 255)) :!label _label
        (`SceneComponent.K2_SetWorldLocation` _labdoor01 (+ (`SceneComponent.K2_GetComponentLocation` _labdoor01) (0.0 0.0 1.0)) false false)
        (set `self.evolDoorPos` (+ _evoldoorpos 1))
        (`KismetSystemLibrary.Delay` 0.008)
        (goto _label)))))

(fn `CloseDoor`)

(fn `UserConstructionScript`)