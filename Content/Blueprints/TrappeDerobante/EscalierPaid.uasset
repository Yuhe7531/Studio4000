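; Staircase actor that starts shifted along its local Y axis and slides back to its placed position after its Paid event fires.
; BeginPlay pushes the root component out by the integer Offset.
; Paid waits briefly, then starts a looping timer on Movement, which steps the root back one unit per tick, counting Offset down and clearing the timer at zero.
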(event `self.ReceiveBeginPlay`
  (`SceneComponent.K2_AddLocalOffset` (`self.DefaultSceneRoot`) (`KismetMathLibrary.MakeVector` 0.0 (`KismetMathLibrary.Conv_IntToDouble` (`self.Offset`))) false false))

(event `self.ReceiveTick`
  (params (DeltaSeconds :type "Float (single-precision)")))

(event `/Game/Blueprints/DATA/BPI.Paid`
  (`KismetSystemLibrary.Delay` 5.0)
  (`KismetSystemLibrary.K2_SetTimer` null "Movement" 0.07 true))

(fn `Movement`
  (if (== (`self.Offset`) 0)
    (`KismetSystemLibrary.K2_ClearTimer` null "Movement")
    (else
      (`SceneComponent.K2_AddLocalOffset` (`self.DefaultSceneRoot`) (0.0 -1.0 0.0) false false)
      (set `self.Offset` (- (`self.Offset`) 1)))))

(fn `UserConstructionScript`)