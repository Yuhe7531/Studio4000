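; BP_Cible is a target actor that reports hits on its mesh to the BP_Socle actors in the level.
; On each component hit, it gathers every BP_Socle and checks its Direction value in a sequence of branches.
; The value selects which north, south, west or east shot message (TirN, TirS, TirO, TirE) is called on all of them.
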(event `self.CibleMesh.OnComponentHit`
  (params (HitComponent :type "PrimitiveComponent Object Reference") (OtherActor :type "Actor Object Reference") (OtherComp :type "PrimitiveComponent Object Reference") (NormalImpulse :type "Vector Structure") (Hit :type "HitResult Structure (by ref)"))
  (bind _outactors (`GameplayStatics.GetAllActorsOfClass` "/Game/Blueprints/Overboard/BP_Socle.BP_Socle_C"))
  (`|ExecutionSequence`
    (:`then_0`
      (if (== (`self.direction`) 1)
        (message `/Game/Blueprints/Overboard/BP_hit.tir_N` _outactors)))
    (:`then_1`
      (if (== (`self.direction`) 2)
        (message `/Game/Blueprints/Overboard/BP_hit.tir_S` _outactors)))
    (:`then_2`
      (if (== (`self.direction`) 3)
        (message `/Game/Blueprints/Overboard/BP_hit.tir_O` _outactors)))
    (:`then_3`
      (if (== (`self.direction`) 4)
        (message `/Game/Blueprints/Overboard/BP_hit.tir_E` _outactors)))))

(fn `UserConstructionScript`)