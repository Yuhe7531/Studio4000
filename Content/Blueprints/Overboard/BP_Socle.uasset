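; BP_Socle is a physics-driven base actor in the Overboard game that gets knocked along the horizontal axes and can be reset.
; Four directional shot events (TirN, TirS, TirO, TirE) each apply a fixed velocity-change impulse to SocleMesh.
; TPSocle zeroes linear velocity on SocleMesh and Strie1, then teleports to SoclePos with zero rotation, targeting the instance found by GetActorOfClass rather than self.
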(event `self.ReceiveBeginPlay`
  (set `self.soclePos` (`self.soclePos`))
  (`GameplayStatics.SetEnableWorldRendering` true))

(event `/Game/Blueprints/Overboard/BP_hit.tir_N`
  (`PrimitiveComponent.AddImpulse` (`self.SocleMesh`) (-350.0 0.0 0.0) "None" true))

(event `/Game/Blueprints/Overboard/BP_hit.tir_S`
  (`PrimitiveComponent.AddImpulse` (`self.SocleMesh`) (350.0 0.0 0.0) "None" true))

(event `/Game/Blueprints/Overboard/BP_hit.tir_O`
  (`PrimitiveComponent.AddImpulse` (`self.SocleMesh`) (0.0 350.0 0.0) "None" true))

(event `/Game/Blueprints/Overboard/BP_hit.tir_E`
  (`PrimitiveComponent.AddImpulse` (`self.SocleMesh`) (0.0 -350.0 0.0) "None" true))

(fn `TP_socle`
  (bind _returnvalue (`GameplayStatics.GetActorOfClass` "BP_Socle_C"))
  (`PrimitiveComponent.SetPhysicsLinearVelocity` (`/Game/Blueprints/Overboard/BP_Socle.SocleMesh` _returnvalue) (0.0 0.0 0.0) false "socle")
  (`PrimitiveComponent.SetPhysicsLinearVelocity` (`/Game/Blueprints/Overboard/BP_Socle.strie1` _returnvalue) (0.0 0.0 0.0) false "socle")
  (`self.K2_TeleportTo` :`self` _returnvalue :`DestLocation` (`/Game/Blueprints/Overboard/BP_Socle.soclePos` _returnvalue)))

(fn `UserConstructionScript`)