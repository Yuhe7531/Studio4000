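; BP_Finish is the end-of-game trigger actor in Overboard.
; When its static mesh is hit by the FirstPersonCharacter, it prints a French congratulation summary on screen for ten seconds.
; The summary reads the character's life, bolt, bullet and cell counts, with cells shown out of 25 and taken from the Saut variable.
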(event `self.StaticMeshComponent.OnComponentHit`
  (params (HitComponent :type "PrimitiveComponent Object Reference") (OtherActor :type "Actor Object Reference") (OtherComp :type "PrimitiveComponent Object Reference") (NormalImpulse :type "Vector Structure") (Hit :type "HitResult Structure (by ref)"))
  ;[1 1 1] Résumé (fin)
  (bind _asfirst_person_character (cast `/Game/Blueprints/FirstPersonCharacter` OtherActor))
  (`KismetSystemLibrary.PrintString` (`KismetStringLibrary.Concat_StrStr` "BRAVO : Vous avez fini le jeu avec :" (`KismetStringLibrary.Concat_StrStr` "Vie :  " (`KismetStringLibrary.Conv_IntToString` (`/Game/Blueprints/FirstPersonCharacter.Vie` _asfirst_person_character)) " -  " "Boulon(s) :  " (`KismetStringLibrary.Conv_IntToString` (`/Game/Blueprints/FirstPersonCharacter.Boulon` _asfirst_person_character)) " -  " "Balle(s) :  " (`KismetStringLibrary.Conv_IntToString` (`/Game/Blueprints/FirstPersonCharacter.Balle` _asfirst_person_character)) " -  " "Cellules :  " (`KismetStringLibrary.Conv_IntToString` (`/Game/Blueprints/FirstPersonCharacter.Saut` _asfirst_person_character)) "/25")) true true (struct :`G` 0.66 :`B` 1.0 :`A` 1.0) 10.0))

(fn `UserConstructionScript`)