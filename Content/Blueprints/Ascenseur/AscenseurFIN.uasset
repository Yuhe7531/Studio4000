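; End-of-level elevator actor that opens its door, closes it and rises, with the fade-out and teleport to the next level only a placeholder print.
; Hits on the opening and closing boxes each fire once, playing duration-scaled timelines that lerp the door between origin and target.
; After closing and a short delay, a third timeline lifts the cabin by a fixed height.
; Door moves are duplicated on the same VersXbas component.
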(event `self.ReceiveBeginPlay`
  (bind _returnvalue (`SceneComponent.K2_GetComponentLocation` (`self.Ascenseur`)))
  (set `self.PositionBasse` _returnvalue)
  (set `self.PositionHaute` (+ _returnvalue (0.0 0.0 2500.0)))
  (set `self.OriginePorteX` (`SceneComponent.K2_GetComponentLocation` (`self.versXbas`)))
  (set `self.OriginePorte-X` (`SceneComponent.K2_GetComponentLocation` (`self.vers-Xbas`))))

(event `self.BoxOuverture.OnComponentHit`
  (params (HitComponent :type "PrimitiveComponent Object Reference") (OtherActor :type "Actor Object Reference") (OtherComp :type "PrimitiveComponent Object Reference") (NormalImpulse :type "Vector Structure") (Hit :type "HitResult Structure (by ref)"))
  (`/Engine/EditorBlueprintResources/StandardMacros.DoOnce` false
    (:`Completed`
      (`TimelineComponent.SetPlayRate` (`self.OuverturePorte`) (/ 1.0 (`self.TempsOuverturePorte`)))
      (bind (_direction _alpha) (`Timeline|OuverturePorte`)
        (:`Update`
          (`SceneComponent.K2_SetWorldLocation` (`self.vers-Xbas`) (`KismetMathLibrary.VLerp` (`self.OriginePorte-X`) (`SceneComponent.K2_GetComponentLocation` (`self.Target-Xbas`)) _alpha) false false)
          (`SceneComponent.K2_SetWorldLocation` (`self.versXbas`) (`KismetMathLibrary.VLerp` (`self.OriginePorteX`) (`SceneComponent.K2_GetComponentLocation` (`self.TargetXbas`)) _alpha) false false))))))

(event `self.BoxFermeture.OnComponentHit`
  (params (HitComponent :type "PrimitiveComponent Object Reference") (OtherActor :type "Actor Object Reference") (OtherComp :type "PrimitiveComponent Object Reference") (NormalImpulse :type "Vector Structure") (Hit :type "HitResult Structure (by ref)"))
  (`/Engine/EditorBlueprintResources/StandardMacros.DoOnce` false
    (:`Completed`
      (`TimelineComponent.SetPlayRate` (`self.FermeturePorte`) (/ 1.0 (`self.TempsOuverturePorte`)))
      (bind (_direction _alpha) (`Timeline|FermeturePorte`)
        (:`Update`
          (`SceneComponent.K2_SetWorldLocation` (`self.vers-Xbas`) (`KismetMathLibrary.VLerp` (`SceneComponent.K2_GetComponentLocation` (`self.Target-Xbas`)) (`self.OriginePorte-X`) _alpha) false false)
          (`SceneComponent.K2_SetWorldLocation` (`self.versXbas`) (`KismetMathLibrary.VLerp` (`SceneComponent.K2_GetComponentLocation` (`self.TargetXbas`)) (`self.OriginePorteX`) _alpha) false false))
        (:`Finished`
          (`KismetSystemLibrary.Delay` 1.0)
          (`TimelineComponent.SetPlayRate` (`self.MonteeAscenseur`) (/ 1.0 (`self.TempsDeplacement`)))
          (bind (_direction_2 _alpha_2) (`Timeline|MonteeAscenseur`)
            (:`Update`
              (`SceneComponent.K2_SetWorldLocation` (`self.Ascenseur`) (`KismetMathLibrary.VLerp` (`self.PositionBasse`) (`self.PositionHaute`) _alpha_2) false false))
            (:`Finished`
              (`KismetSystemLibrary.PrintString` "Ecran noir progressif + TP vers level suivant"))))))))

(fn `UserConstructionScript`)