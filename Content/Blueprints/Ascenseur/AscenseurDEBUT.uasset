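; AscenseurDEBUT is a starting elevator that rises automatically on BeginPlay, then opens its door at the top.
; A timeline lerps the Ascenseur component from its initial position to a fixed height above it, scaled by TempsDeplacement.
; After a short delay, a second timeline, scaled by TempsOuverturePorte, slides VersXhaut to TargetXhaut's location.
; The door origin and movement calls are duplicated on VersXhaut, so only that door component moves.
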(event `self.ReceiveBeginPlay`
  (bind _returnvalue (`SceneComponent.K2_GetComponentLocation` (`self.Ascenseur`)))
  (set `self.PositionBasse` _returnvalue)
  (set `self.PositionHaute` (+ _returnvalue (0.0 0.0 2500.0)))
  (set `self.OriginePorteX` (`SceneComponent.K2_GetComponentLocation` (`self.versXhaut`)))
  (set `self.OriginePorte-X` (`SceneComponent.K2_GetComponentLocation` (`self.vers-Xhaut`)))
  (`TimelineComponent.SetPlayRate` (`self.MonteeAscenseur`) (/ 1.0 (`self.TempsDeplacement`)))
  (bind (_direction _alpha) (`Timeline|MonteeAscenseur`)
    (:`Update`
      (`SceneComponent.K2_SetWorldLocation` (`self.Ascenseur`) (`KismetMathLibrary.VLerp` (`self.PositionBasse`) (`self.PositionHaute`) _alpha) false false))
    (:`Finished`
      (`KismetSystemLibrary.Delay` 1.0)
      (`TimelineComponent.SetPlayRate` (`self.OuverturePorte`) (/ 1.0 (`self.TempsOuverturePorte`)))
      (bind (_direction_2 _alpha_2) (`Timeline|OuverturePorte`)
        (:`Update`
          (`SceneComponent.K2_SetWorldLocation` (`self.vers-Xhaut`) (`KismetMathLibrary.VLerp` (`self.OriginePorte-X`) (`SceneComponent.K2_GetComponentLocation` (`self.Target-Xhaut`)) _alpha_2) false false)
          (`SceneComponent.K2_SetWorldLocation` (`self.versXhaut`) (`KismetMathLibrary.VLerp` (`self.OriginePorteX`) (`SceneComponent.K2_GetComponentLocation` (`self.TargetXhaut`)) _alpha_2) false false))))))

(fn `UserConstructionScript`)